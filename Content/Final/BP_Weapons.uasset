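; Weapon pickup actor that the first-person player collects through an Interact event.
; The construction script picks the mesh from WeaponType, using either a gun model or a scaled-down knife.
; Box overlaps create a W_Interact hint in a widget component and animate it popping in and out.
; Interact flags the character's PickedGun, destroys the pickup, stores the weapon type in GM_Gm and calls the character's picked-up dispatcher.
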(event `self.ReceiveBeginPlay`
  (bind _asbp_first_person_character (cast `/Game/FirstPerson/Blueprints/BP_FirstPersonCharacter` (`GameplayStatics.GetPlayerCharacter` 0)))
  (set `self.As BP First Person Character` _asbp_first_person_character)
  (bind _asgm_gm (cast `/Game/Final/GM_Gm` (`GameplayStatics.GetGameMode`)))
  (set `self.As GM Gm` _asgm_gm))

(event `/Game/Final/BPI_Interact.Interact`
  (bind _as_bp_first_person_character (`self.As BP First Person Character`))
  (bind _as_gm_gm (`self.As GM Gm`))
  (set `/Game/FirstPerson/Blueprints/BP_FirstPersonCharacter.PickedGun?` true _as_bp_first_person_character)
  (`self.K2_DestroyActor`)
  (if (`|EnumEquality` (`self.WeaponType`) "NewEnumerator1")
    (set `/Game/Final/GM_Gm.Weapons` "NewEnumerator1" _as_gm_gm)
    (`/Game/FirstPerson/Blueprints/BP_FirstPersonCharacter.DP_PickedUp` _as_bp_first_person_character :!label _label)
    (elif (`|EnumEquality` (`self.WeaponType`) "NewEnumerator2")
      (set `/Game/Final/GM_Gm.Weapons` "NewEnumerator2" _as_gm_gm)
      (goto _label))))

(event `self.Box.OnComponentBeginOverlap`
  (params (OverlappedComponent :type "PrimitiveComponent Object Reference") (OtherActor :type "Actor Object Reference") (OtherComp :type "PrimitiveComponent Object Reference") (OtherBodyIndex :type Integer) (bFromSweep :type Boolean) (SweepResult :type "HitResult Structure (by ref)"))
  (bind _widget (`self.Widget`))
  (bind _returnvalue (`|CreateWidget` "/Game/Final/Widgets/W_Interact.W_Interact_C"))
  (bind _output_get (set `self.NewVar` _returnvalue))
  (`WidgetComponent.SetWidget` _widget _output_get)
  (`SceneComponent.SetVisibility` _widget true false)
  (bind _newvar (`self.NewVar`)
    (:`then`
      (if (not (`self.HintVisible`))
        (`UserWidget.PlayAnimation` _newvar (`/Game/Final/Widgets/W_Interact.PopUp` _newvar) 0.0 1 "Forward" 2.0 false)
        (set `self.HintVisible` true)))
    (:`else`)))

(event `self.Box.OnComponentEndOverlap`
  (params (OverlappedComponent :type "PrimitiveComponent Object Reference") (OtherActor :type "Actor Object Reference") (OtherComp :type "PrimitiveComponent Object Reference") (OtherBodyIndex :type Integer))
  (bind _newvar (`self.NewVar`)
    (:`then`
      (if (`self.HintVisible`)
        (`UserWidget.PlayAnimation` _newvar (`/Game/Final/Widgets/W_Interact.PopOut` _newvar) 0.0 1 "Forward" 2.0 false)
        (set `self.HintVisible` false)))
    (:`else`)))

(fn `UserConstructionScript`
  (bind _weapontype (`self.WeaponType`))
  (if (== _weapontype 1)
    (`StaticMeshComponent.SetStaticMesh` (`self.StaticMesh`) "/Game/Fab/Megascans/3D/Axe_ubglcesiw/High/ubglcesiw_tier_1.ubglcesiw_tier_1")
    (elif (== _weapontype 2)
      (`StaticMeshComponent.SetStaticMesh` (`self.StaticMesh`) "/Game/Fab/Knife/knife.knife")
      (`SceneComponent.SetRelativeScale3D` (`self.StaticMesh`) (* (`SceneComponent.RelativeScale3D` (`self.StaticMesh`)) 0.1)))))