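; BP_Medkit is a medkit pickup that restores 25 health to the player's first-person character when interacted with, then destroys itself.
; BeginPlay caches the player character for the heal call.
; A sphere overlap creates a W_Interact prompt in a widget component and plays its pop-up animation, and end overlap plays the pop-out, with a HintVisible flag preventing repeated animations.
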(event `self.ReceiveBeginPlay`
  (bind _asbp_first_person_character (cast `/Game/FirstPerson/Blueprints/BP_FirstPersonCharacter` (`GameplayStatics.GetPlayerCharacter` 0)))
  (set `self.As BP First Person Character` _asbp_first_person_character))

(event `/Game/Final/BPI_Interact.Interact`
  (`/Game/FirstPerson/Blueprints/BP_FirstPersonCharacter.HealthUpdate` (`self.As BP First Person Character`) 25.0)
  (`self.K2_DestroyActor`))

(event `self.Sphere.OnComponentBeginOverlap`
  (params (OverlappedComponent :type "PrimitiveComponent Object Reference") (OtherActor :type "Actor Object Reference") (OtherComp :type "PrimitiveComponent Object Reference") (OtherBodyIndex :type Integer) (bFromSweep :type Boolean) (SweepResult :type "HitResult Structure (by ref)"))
  (bind _widget (`self.Widget`))
  (bind _returnvalue (`|CreateWidget` "/Game/Final/Widgets/W_Interact.W_Interact_C"))
  (bind _output_get (set `self.InteractWidget` _returnvalue))
  (`WidgetComponent.SetWidget` _widget _output_get)
  (`SceneComponent.SetVisibility` _widget true false)
  (bind _interactwidget (`self.InteractWidget`)
    (:`then`
      (if (not (`self.HintVisible`))
        (`UserWidget.PlayAnimation` _interactwidget (`/Game/Final/Widgets/W_Interact.PopUp` _interactwidget) 0.0 1 "Forward" 2.0 false)
        (set `self.HintVisible` true)))
    (:`else`)))

(event `self.Sphere.OnComponentEndOverlap`
  (params (OverlappedComponent :type "PrimitiveComponent Object Reference") (OtherActor :type "Actor Object Reference") (OtherComp :type "PrimitiveComponent Object Reference") (OtherBodyIndex :type Integer))
  (bind _interactwidget (`self.InteractWidget`)
    (:`then`
      (if (`self.HintVisible`)
        (`UserWidget.PlayAnimation` _interactwidget (`/Game/Final/Widgets/W_Interact.PopOut` _interactwidget) 0.0 1 "Forward" 2.0 false)
        (set `self.HintVisible` false)))
    (:`else`)))

(fn `UserConstructionScript`)